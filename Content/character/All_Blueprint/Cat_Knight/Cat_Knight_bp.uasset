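; Cat Knight player character for a charge-jump platformer, moved by physics forces on its capsule, with a ground trace and X-speed clamp each Tick.
; Holding Jump builds force on a looping timer and publishes charge to a parameter collection; release launches if grounded.
; Escape uses four diagonal traces to detect being stuck, then retries teleports around the pre-jump location.
; It also handles damage, the fail widget and a timed whole-map camera.
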(event `self.ReceiveAnyDamage`
  (params (Damage :type "Float (single-precision)") (DamageType :type "DamageType Object Reference") (InstigatedBy :type "Controller Object Reference") (DamageCauser :type "Actor Object Reference"))
  (bind _returnvalue (`KismetMaterialLibrary.GetScalarParameterValue` "/Game/User_Interface/local_DB/TEMP_DATA_local.TEMP_DATA_local" "currenthp"))
  (`KismetMaterialLibrary.SetScalarParameterValue` "/Game/User_Interface/local_DB/TEMP_DATA_local.TEMP_DATA_local" "currenthp" (- _returnvalue Damage))
  (bind _returnvalue_2 (`KismetMaterialLibrary.GetScalarParameterValue` "/Game/User_Interface/local_DB/TEMP_DATA_local.TEMP_DATA_local" "currenthp"))
  (if (== _returnvalue_2 0.0)
    (bind _returnvalue_3 (`|CreateWidget` "/Game/User_Interface/FAIL_.FAIL__C"))
    (`UserWidget.AddToViewport` _returnvalue_3 0)))

(event `Reset_Camera`
  (`PlayerController.SetViewTargetWithBlend` (`GameplayStatics.GetPlayerController` 0) (`self.Origin_Camera`) 1.0 "VTBlend_Linear" 0.0 false)
  (set `self.Can_Switch_Camera` true))

(event `self.ReceiveTick`
  (params (DeltaSeconds :type "Float (single-precision)"))
  (bind _returnvalue (`self.K2_GetActorLocation`))
  (bind (_x _y _z) (`KismetMathLibrary.BreakVector3f` (`self.GetVelocity`)))
  (`PrimitiveComponent.SetAllPhysicsLinearVelocity` (`self.CapsuleComponent`) (`KismetMathLibrary.MakeVector` (`KismetMathLibrary.FClamp` _x -400.0 400.0) _y _z) false)
  (bind (_outhit _returnvalue_2) (`KismetSystemLibrary.LineTraceSingle` _returnvalue (- _returnvalue (0.0 0.0 100.0)) "TraceTypeQuery1"))
  (if _returnvalue_2
    (set `self.IsOnGround` true)
    (else
      (set `self.IsOnGround` false))))

(event `InputAction|SeeWholeMap`
  (params (Key :type "Key Structure"))
  (:`Pressed`
    (if (`self.Can_Switch_Camera`)
      (set `self.Can_Switch_Camera` false)
      (set `self.Origin_Camera` (`Controller.GetViewTarget` (`GameplayStatics.GetPlayerController` 0)))
      (`KismetSystemLibrary.K2_ClearAndInvalidateTimerHandle` (`self.CameraSwitch_TimerHandle`))
      (bind _outactors (`GameplayStatics.GetAllActorsOfClass` "/Game/character/All_Blueprint/character/FixedCamera.FixedCamera_C"))
      (`PlayerController.SetViewTargetWithBlend` (`GameplayStatics.GetPlayerController` 0) (`|GetArrayItem` _outactors) 1.0 "VTBlend_Linear" 0.0 false)
      (bind _returnvalue (`KismetSystemLibrary.K2_SetTimerDelegate` (delegate `Reset_Camera`) 3.0))
      (set `self.CameraSwitch_TimerHandle` _returnvalue))))

(event `InputAxis|Move_Right`
  (params (AxisValue :type "Float (single-precision)"))
  (if (`self.Is_Jumping`)
    _
    (elif (`self.IsOnGround`)
      (`PrimitiveComponent.AddForce` (`self.CapsuleComponent`) (`KismetMathLibrary.MakeVector` (* AxisValue 1000.0)) "None" true))))

(event `InputAction|Jump`
  (params (Key :type "Key Structure"))
  (:`Pressed`
    (set `self.Prev_Location` (`self.K2_GetActorLocation`))
    (set `self.Is_Jumping` true)
    (bind _returnvalue (`KismetSystemLibrary.K2_SetTimerDelegate` (delegate `ChargeJump`) 0.1 true))
    (set `self.Charge Time Handle` _returnvalue))
  (:`Released`
    (`KismetSystemLibrary.K2_ClearAndInvalidateTimerHandle` (`self.Charge Time Handle`))
    (`KismetSystemLibrary.PrintString` (`KismetStringLibrary.Conv_DoubleToString` (`self.JumpCharge`)) true true (struct :`G` 1.0 :`B` 0.310475 :`A` 1.0))
    (if (`self.IsOnGround`)
      (`PrimitiveComponent.AddForce` (`self.CapsuleComponent`) (`KismetMathLibrary.MakeVector` (`self.RightCharge`) 0.0 (`self.JumpCharge`)) "None" true)
      (`KismetSystemLibrary.PrintString` (`KismetStringLibrary.Conv_DoubleToString` (`self.RightCharge`)) true true (struct :`G` 1.0 :`B` 0.311617 :`A` 1.0))
      (set `self.RightCharge` 0.0)
      (set `self.JumpCharge` 16000.0)
      (set `self.add_charge` 0.0)
      (set `self.Is_Jumping` false)
      (`KismetMaterialLibrary.SetScalarParameterValue` "/Game/User_Interface/Material_for_data/TEMP_DATA.TEMP_DATA" "Charge"))))

(event `ChargeJump`
  (bind _returnvalue (`KismetMathLibrary.FClamp` (+ (`self.JumpCharge`) (`self.add_charge`)) 0.0 60000.0))
  (set `self.RightCharge` (`KismetMathLibrary.FClamp` (+ (`self.RightCharge`) (* (stale `InputAxis|Move_Right` AxisValue) 2000.0)) -20000.0 20000.0))
  (set `self.add_charge` (+ (`self.add_charge`) 1000.0))
  (bind _output_get (set `self.JumpCharge` _returnvalue))
  (`KismetSystemLibrary.PrintString` (`KismetStringLibrary.Conv_DoubleToString` _output_get))
  (`KismetMaterialLibrary.SetScalarParameterValue` "/Game/User_Interface/Material_for_data/TEMP_DATA.TEMP_DATA" "Charge" (/ _returnvalue 60000.0)))

(event `InputAction|Escape`
  (params (Key :type "Key Structure"))
  (:`Pressed`
    (`self.CheckIsStucked`))
  (:`Released`
    (if (`self.IsStucked`)
      (`self.K2_TeleportTo` (`self.Prev_Location`))
      (`self.CheckIsStucked`)
      (if (`self.IsStucked`)
        (`KismetSystemLibrary.PrintString` "First Try Failed..." true true (struct :`R` 1.0 :`B` 0.066667 :`A` 1.0))
        (`KismetSystemLibrary.Delay` 2.0)
        (if (> (`self.Condition(Step on Left Edge)`) (`self.Condition(Step on Right Edge)`))
          (`self.K2_TeleportTo` (+ (`self.Prev_Location`) (-20.0 0.0 20.0)))
          (`self.CheckIsStucked`)
          (if (`self.IsStucked`)
            (`KismetSystemLibrary.PrintString` "Second Try Failed..." true true (struct :`R` 1.0 :`B` 0.065472 :`A` 1.0))
            (`KismetSystemLibrary.Delay` 2.0)
            (`self.K2_TeleportTo` (+ (`self.Prev_Location`) (20.0 0.0 20.0)))
            (`self.CheckIsStucked`)
            (if (`self.IsStucked`)
              (`KismetSystemLibrary.PrintString` "Third Try Failed..." true true (struct :`R` 1.0 :`B` 0.065472 :`A` 1.0))
              (`KismetSystemLibrary.Delay` 2.0)
              (`self.K2_TeleportTo` (+ (`self.Prev_Location`) (20.0 0.0 -20.0)))
              (`self.CheckIsStucked`)
              (if (`self.IsStucked`)
                (`KismetSystemLibrary.PrintString` "Fourth Try Failed..." true true (struct :`R` 1.0 :`B` 0.065472 :`A` 1.0))
                (`KismetSystemLibrary.Delay` 2.0)
                (`self.K2_TeleportTo` (+ (`self.Prev_Location`) (-20.0 0.0 -20.0)))
                (`self.CheckIsStucked`)
                (if (`self.IsStucked`)
                  (`KismetSystemLibrary.PrintString` "All tries failed..." true true (struct :`R` 1.0 :`B` 0.065472 :`A` 1.0))
                  (`KismetSystemLibrary.Delay` 1.0)
                  (`KismetSystemLibrary.PrintString` "Wait a second..." true true (struct :`R` 1.0 :`B` 0.066667 :`A` 1.0))
                  (`KismetSystemLibrary.Delay` 3.0)
                  (`self.K2_TeleportTo` (0.0 0.0 0.0))
                  (`KismetSystemLibrary.PrintString` "Sorry, I can't help you. \nBut I hope you play well:))))" true true (struct :`R` 1.0 :`B` 0.066667 :`A` 1.0))
                  (else
                    (`PrimitiveComponent.SetAllPhysicsLinearVelocity` (`self.CapsuleComponent`) (0.0 0.0 0.0) false)
                    (`KismetSystemLibrary.PrintString` "Lat Escape Suceessfully!!!" true true (struct :`R` 1.0 :`B` 0.066667 :`A` 1.0))))
                (else
                  (`PrimitiveComponent.SetAllPhysicsLinearVelocity` (`self.CapsuleComponent`) (0.0 0.0 0.0) false)
                  (`KismetSystemLibrary.PrintString` "Fourth Escape Suceessfully!!!" true true (struct :`R` 1.0 :`B` 0.066667 :`A` 1.0))))
              (else
                (`PrimitiveComponent.SetAllPhysicsLinearVelocity` (`self.CapsuleComponent`) (0.0 0.0 0.0) false)
                (`KismetSystemLibrary.PrintString` "Third Escape Suceessfully!!!" true true (struct :`R` 1.0 :`B` 0.066667 :`A` 1.0))))
            (else
              (`PrimitiveComponent.SetAllPhysicsLinearVelocity` (`self.CapsuleComponent`) (0.0 0.0 0.0) false)
              (`KismetSystemLibrary.PrintString` "Second Escape Suceessfully!!!" true true (struct :`R` 1.0 :`B` 0.066667 :`A` 1.0))))
          (else
            (`self.K2_TeleportTo` (+ (`self.Prev_Location`) (20.0 0.0 20.0)))
            (`self.CheckIsStucked`)
            (if (`self.IsStucked`)
              (`KismetSystemLibrary.PrintString` "Second Try Failed..." true true (struct :`R` 1.0 :`B` 0.065472 :`A` 1.0))
              (`KismetSystemLibrary.Delay` 2.0)
              (`self.K2_TeleportTo` (+ (`self.Prev_Location`) (-20.0 0.0 20.0)))
              (`self.CheckIsStucked`)
              (if (`self.IsStucked`)
                (`KismetSystemLibrary.PrintString` "Third Try Failed..." true true (struct :`R` 1.0 :`B` 0.065472 :`A` 1.0))
                (`KismetSystemLibrary.Delay` 2.0)
                (`self.K2_TeleportTo` (+ (`self.Prev_Location`) (20.0 0.0 -20.0)))
                (`self.CheckIsStucked`)
                (if (`self.IsStucked`)
                  (`KismetSystemLibrary.PrintString` "Fourth Try Failed..." true true (struct :`R` 1.0 :`B` 0.065472 :`A` 1.0))
                  (`KismetSystemLibrary.Delay` 2.0)
                  (`self.K2_TeleportTo` (+ (`self.Prev_Location`) (-20.0 0.0 -20.0)))
                  (`self.CheckIsStucked`)
                  (if (`self.IsStucked`)
                    (`KismetSystemLibrary.PrintString` "All tries failed..." true true (struct :`R` 1.0 :`B` 0.065472 :`A` 1.0))
                    (`KismetSystemLibrary.Delay` 1.0)
                    (`KismetSystemLibrary.PrintString` "Wait a second..." true true (struct :`R` 1.0 :`B` 0.066667 :`A` 1.0))
                    (bind _astoast_knight_controller_bp (cast `/Game/character/Gamemode/Toast_Knight_controller_bp` (`GameplayStatics.GetPlayerController` 0)))
                    (`KismetSystemLibrary.Delay` 3.0)
                    (`self.K2_TeleportTo` (`/Game/character/Gamemode/Toast_Knight_controller_bp.Initial_Location` (`|GetArrayItem` (`|MakeArray` _astoast_knight_controller_bp))))
                    (`KismetSystemLibrary.PrintString` "Sorry, I can't help you. \nBut I hope you play well:))))" true true (struct :`R` 1.0 :`B` 0.066667 :`A` 1.0))
                    (else
                      (`PrimitiveComponent.SetAllPhysicsLinearVelocity` (`self.CapsuleComponent`) (0.0 0.0 0.0) false)
                      (`KismetSystemLibrary.PrintString` "Lat Escape Suceessfully!!!" true true (struct :`R` 1.0 :`B` 0.066667 :`A` 1.0))))
                  (else
                    (`PrimitiveComponent.SetAllPhysicsLinearVelocity` (`self.CapsuleComponent`) (0.0 0.0 0.0) false)
                    (`KismetSystemLibrary.PrintString` "Fourth Escape Suceessfully!!!" true true (struct :`R` 1.0 :`B` 0.066667 :`A` 1.0))))
                (else
                  (`PrimitiveComponent.SetAllPhysicsLinearVelocity` (`self.CapsuleComponent`) (0.0 0.0 0.0) false)
                  (`KismetSystemLibrary.PrintString` "Third Escape Suceessfully!!!" true true (struct :`R` 1.0 :`B` 0.066667 :`A` 1.0))))
              (else
                (`PrimitiveComponent.SetAllPhysicsLinearVelocity` (`self.CapsuleComponent`) (0.0 0.0 0.0) false)
                (`KismetSystemLibrary.PrintString` "Second Escape Suceessfully!!!" true true (struct :`R` 1.0 :`B` 0.066667 :`A` 1.0))))))
        (else
          (`PrimitiveComponent.SetAllPhysicsLinearVelocity` (`self.CapsuleComponent`) (0.0 0.0 0.0) false)
          (`KismetSystemLibrary.PrintString` "First Escape Suceessfully!!!" true true (struct :`R` 1.0 :`B` 0.066667 :`A` 1.0))))
      (else
        (`KismetSystemLibrary.PrintString` "Escape Failed!!!")))))

(fn `CheckIsStucked`
  (bind _returnvalue (`self.K2_GetActorLocation`))
  (bind _returnvalue_2 (`self.K2_GetActorLocation`))
  (bind _returnvalue_3 (`self.K2_GetActorLocation`))
  (bind _returnvalue_4 (`self.K2_GetActorLocation`))
  (set `self.IsStucked` false)
  (set `self.Condition(Step on Left Edge)` 0)
  (set `self.Condition(Step on Right Edge)` 0)
  (bind (_outhit _returnvalue_5) (`KismetSystemLibrary.LineTraceSingle` :`Start` _returnvalue_2 :`End` (+ _returnvalue_2 (-20.0 0.0 -20.0)) :`TraceChannel` "TraceTypeQuery1" :`DrawDebugType` "ForOneFrame"))
  (bind (_outhit_2 _returnvalue_6) (`KismetSystemLibrary.LineTraceSingle` :`Start` _returnvalue_3 :`End` (+ _returnvalue_3 (20.0 0.0 -20.0)) :`TraceChannel` "TraceTypeQuery1" :`DrawDebugType` "ForOneFrame"))
  (bind (_outhit_3 _returnvalue_7) (`KismetSystemLibrary.LineTraceSingle` :`Start` _returnvalue_4 :`End` (+ _returnvalue_4 (-20.0 0.0 20.0)) :`TraceChannel` "TraceTypeQuery1" :`DrawDebugType` "ForOneFrame"))
  (bind (_outhit_4 _returnvalue_8) (`KismetSystemLibrary.LineTraceSingle` :`Start` _returnvalue :`End` (+ _returnvalue (20.0 0.0 20.0)) :`TraceChannel` "TraceTypeQuery1" :`DrawDebugType` "ForOneFrame"))
  (if _returnvalue_5
    (if _returnvalue_6
      (if _returnvalue_7
        (if _returnvalue_8
          (`KismetSystemLibrary.PrintString` "Are you're stucked in block!?!?" true true (struct :`R` 0.998508 :`G` 1.0 :`A` 1.0))
          (set `self.IsStucked` true)
          (else
            (`KismetSystemLibrary.PrintString` "Detected No Stucked(You are at the left corner!!!)" true true (struct :`R` 0.998508 :`G` 1.0 :`A` 1.0))))
        (elif _returnvalue_8
          (`KismetSystemLibrary.PrintString` "Detected No Stucked(You are at the right corner!!!)" true true (struct :`R` 0.998508 :`G` 1.0 :`A` 1.0))
          (else
            (`KismetSystemLibrary.PrintString` "Detected No Stucked(You are on the plain platform!!!)" true true (struct :`R` 0.998508 :`G` 1.0 :`A` 1.0)))))
      (elif _returnvalue_7
        (`KismetSystemLibrary.PrintString` "Detected No Stucked" true true (struct :`R` 0.998508 :`G` 1.0 :`A` 1.0))
        (else
          (set `self.IsStucked` true)
          (set `self.Condition(Step on Left Edge)` 1)
          (`KismetSystemLibrary.PrintString` "Detected Stucked..." true true (struct :`R` 0.998508 :`G` 1.0 :`A` 1.0) 3.0 :!label _label))))
    (elif _returnvalue_6
      (if _returnvalue_8
        (`KismetSystemLibrary.PrintString` "Detected No Stucked" true true (struct :`R` 0.998508 :`G` 1.0 :`A` 1.0))
        (else
          (set `self.IsStucked` true)
          (set `self.Condition(Step on Right Edge)` 1)
          (goto _label)))
      (elif _returnvalue_7
        (if _returnvalue_8
          (`KismetSystemLibrary.PrintString` "Detected No Stucked(You are below the roof!!!)" true true (struct :`R` 0.998508 :`G` 1.0 :`A` 1.0))
          (else
            (`KismetSystemLibrary.PrintString` "Maybe you're stucked at the left top???" true true (struct :`R` 0.998508 :`G` 1.0 :`A` 1.0))
            (set `self.IsStucked` true)))
        (elif _returnvalue_8
          (`KismetSystemLibrary.PrintString` "Maybe you're stucked at the right top???" true true (struct :`R` 0.998508 :`G` 1.0 :`A` 1.0))
          (set `self.IsStucked` true)
          (else
            (`KismetSystemLibrary.PrintString` "Are you  in the air???" true true (struct :`R` 0.998508 :`G` 1.0 :`A` 1.0))))))))

(fn `JumpRelease`)

(fn `UserConstructionScript`)