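; YinYung_Knight is a side-moving player character with a hold-to-charge jump, viewed through the level's FixedCamera.
; The horizontal axis applies acceleration-based force on the capsule, with X velocity clamped while falling.
; Holding Jump runs a looping timer that grows the charge and writes it to the TEMP_DATA parameter collection.
; Releasing stops the timer, applies the charge as upward force and resets it, with debug prints of the value.
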(event `self.ReceiveBeginPlay`
  (bind _outactors (`GameplayStatics.GetAllActorsOfClass` "/Game/character/All_Blueprint/character/FixedCamera.FixedCamera_C"))
  (`PlayerController.SetViewTargetWithBlend` (`GameplayStatics.GetPlayerController` 0) (`|GetArrayItem` _outactors) 0.0 "VTBlend_Linear" 0.0 false))

(event `InputAxis|Move_Right`
  (params (AxisValue :type "Float (single-precision)"))
  (bind _maxairspeed (`self.MaxAirSpeed`))
  (`PrimitiveComponent.AddForce` (`self.CapsuleComponent`) (`KismetMathLibrary.MakeVector` (* AxisValue 1000.0)) "None" true)
  (set `self.MaxAirSpeed` 200.0)
  (if (`NavMovementComponent.IsFalling` (`self.CharacterMovement`))
    (set `MovementComponent.Velocity` (`KismetMathLibrary.MakeVector` (`KismetMathLibrary.FClamp` (.x (`self.GetVelocity`)) (- 0.0 _maxairspeed) _maxairspeed) (.y (`self.GetVelocity`)) (.z (`self.GetVelocity`))) (`self.CharacterMovement`))))

(event `InputAction|Jump`
  (params (Key :type "Key Structure"))
  (:`Pressed`
    (bind _returnvalue (`KismetSystemLibrary.K2_SetTimerDelegate` (delegate `ChargeJump`) 0.1 true))
    (set `self.Charge Time Handle` _returnvalue))
  (:`Released`
    (`KismetSystemLibrary.K2_ClearAndInvalidateTimerHandle` (`self.Charge Time Handle`))
    (`KismetSystemLibrary.PrintString` (`KismetStringLibrary.Conv_DoubleToString` (`self.JumpCharge`)) true true (struct :`G` 1.0 :`B` 0.310475 :`A` 1.0))
    (`PrimitiveComponent.AddForce` (`self.CapsuleComponent`) (`KismetMathLibrary.MakeVector` 0.0 0.0 (`self.JumpCharge`)) "None" true)
    (bind _output_get (set `self.JumpCharge` 0.0))
    (`KismetMaterialLibrary.SetScalarParameterValue` "/Game/User_Interface/Material_for_data/TEMP_DATA.TEMP_DATA" "Charge" _output_get)))

(event `ChargeJump`
  (bind _output_get (set `self.JumpCharge` (+ (`self.JumpCharge`) 1500.0)))
  (`KismetSystemLibrary.PrintString` (`KismetStringLibrary.Conv_DoubleToString` _output_get))
  (`KismetMaterialLibrary.SetScalarParameterValue` "/Game/User_Interface/Material_for_data/TEMP_DATA.TEMP_DATA" "Charge" (/ _output_get 150000.0)))

(fn `UserConstructionScript`)