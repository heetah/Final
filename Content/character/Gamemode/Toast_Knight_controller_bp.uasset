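; Player controller for the Toast Knight game mode that swaps in the selected character at BeginPlay, after storing its initial focal location.
; Switch_Character destroys the current pawn, then uses the slider value from the MyData game instance to index the game mode's SpawnArray.
; It spawns that class at the controller's own location and rotation and has player controller 0 possess it, printing a message if either cast fails.
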(event `self.ReceiveBeginPlay`
  (set `self.Initial_Location` (`self.GetFocalLocation`))
  (`self.Switch_Character`))

(event `Switch_Character`
  (`self.K2_DestroyActor` (`self.K2_GetPawn`))
  (bind _asmy_data (cast `/Game/User_Interface/Material_for_data/MyData` (`GameplayStatics.GetGameInstance`))
    (:`then`
      (bind _astoast_knight_gamemode_bp (cast `/Game/character/Gamemode/Toast_Knight_gamemode_bp` (`GameplayStatics.GetGameMode`))
        (:`then`
          (bind _returnvalue (`|SpawnActorFromClass` (`|GetArrayItem` (`/Game/character/Gamemode/Toast_Knight_gamemode_bp.SpawnArray` _astoast_knight_gamemode_bp) (`/Game/User_Interface/Material_for_data/MyData.SLIDER_FOR_PLAY` (`|GetArrayItem` (`|MakeArray` _asmy_data)))) (`KismetMathLibrary.MakeTransform` (`self.K2_GetActorLocation`) (`self.K2_GetActorRotation`)) "Undefined" "OverrideRootScale" null null))
          (bind _aspawn (cast `Pawn` _returnvalue))
          (`self.Possess` (`GameplayStatics.GetPlayerController` 0) _aspawn))
        (:`CastFailed`
          (`KismetSystemLibrary.PrintString` "Cast Gamemode Failed" true true (struct :`R` 1.0 :`B` 0.070606 :`A` 1.0)))))
    (:`CastFailed`
      (`KismetSystemLibrary.PrintString` "Cast My_Data Failed" true true (struct :`R` 1.0 :`B` 0.070606 :`A` 1.0)))))

(fn `UserConstructionScript`)