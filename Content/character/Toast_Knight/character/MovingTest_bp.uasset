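; Movement test Blueprint for the Toast Knight, a sprite pawn that moves along world X and jumps, viewed through a fixed camera set at BeginPlay.
; Holding Jump builds charge on a looping timer, and releasing it applies an upward velocity impulse scaled by that uncapped charge.
; Tick applies manual gravity to the PaperSprite and traces downward to set IsOnGround, which is never cleared or used to gate jumping.
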(event `self.ReceiveBeginPlay`
  (bind _outactors (`GameplayStatics.GetAllActorsOfClass` "/Game/character/Toast_Knight/character/FixedCamera.FixedCamera_C"))
  (`PlayerController.SetViewTargetWithBlend` (`GameplayStatics.GetPlayerController` 0) (`|GetArrayItem` _outactors) 0.0 "VTBlend_Linear" 0.0 false))

(event `InputAxis|Move_Right`
  (params (AxisValue :type "Float (single-precision)"))
  (`self.AddMovementInput` (1.0 0.0 0.0) (* AxisValue 3.0)))

(event `InputAction|Jump`
  (params (Key :type "Key Structure"))
  (:`Pressed`
    (`KismetSystemLibrary.K2_SetTimer` null "ChargeJump" 0.1 true))
  (:`Released`
    (`self.JumpRelease`)
    (`PrimitiveComponent.AddImpulse` (`self.PaperSprite`) (* (`self.JumpCharge`) (0.0 0.0 1000.0)) "None" true)
    (set `self.JumpCharge` 0.0)))

(event `ChargeJump`
  (set `self.JumpCharge` (+ (`self.JumpCharge`) 0.1)))

(event `JumpRelease`
  (`KismetSystemLibrary.K2_ClearTimer` null "ChargeJump"))

(event `self.ReceiveTick`
  (params (DeltaSeconds :type "Float (single-precision)"))
  (`PrimitiveComponent.AddForce` (`self.PaperSprite`) (0.0 0.0 -980.0) "None" true)
  (bind (_outhits _returnvalue) (`KismetSystemLibrary.LineTraceMulti` (`self.K2_GetActorLocation`) (+ (`self.K2_GetActorLocation`) (0.0 0.0 -50.0)) "TraceTypeQuery1"))
  (if _returnvalue
    (set `self.IsOnGround` true)))

(fn `UserConstructionScript`)