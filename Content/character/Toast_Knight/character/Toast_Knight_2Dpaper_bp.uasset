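; Toast Knight 2D Paper character that the player launches by dragging and releasing the mouse.
; Fire press stores the start position, and Tick sets CanFire while the left button is held and the character is nearly still.
; Release applies the scaled drag as an X/Z velocity-change impulse, opposite the drag horizontally but following it vertically, as screen Y is not inverted.
; CanFire is never reset, so later releases can launch mid-motion.
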(event `self.ReceiveBeginPlay`
  ;[1 1 1] 增加推動
  (`self.EnableInput` (`GameplayStatics.GetPlayerController` 0)))

(event `InputAction|Fire`
  (params (Key :type "Key Structure"))
  ;[1 1 1] 增加推動
  (:`Pressed`
    (bind _returnvalue (`WidgetLayoutLibrary.GetMousePositionOnViewport`))
    (bind _output_get (set `self.Initial初始滑鼠位置` _returnvalue))))

(event `self.ReceiveTick`
  (params (DeltaSeconds :type "Float (single-precision)"))
  ;[1 1 1] 增加推動
  (if (`PlayerController.IsInputKeyDown` (`GameplayStatics.GetPlayerController` 0) "LeftMouseButton")
    (if (< (`KismetMathLibrary.VSize` (`self.GetVelocity`)) 1.0)
      (set `self.Can Fire` true)
      (bind _returnvalue (`WidgetLayoutLibrary.GetMousePositionOnViewport`))
      (set `self.Current目前滑鼠位置` _returnvalue))))

(event `InputAction|Fire`
  (params (Key :type "Key Structure"))
  ;[1 1 1] 增加推動
  (:`Released`
    (if (`self.Can Fire`)
      (bind _returnvalue (`WidgetLayoutLibrary.GetMousePositionOnViewport`))
      (bind _output_get (set `self.Current目前滑鼠位置` _returnvalue))
      (bind (_x _y) (`KismetMathLibrary.BreakVector2D` (- (stale _output_get) _output_get)))
      (`CharacterMovementComponent.AddImpulse` (`self.CharacterMovement`) (* (`KismetMathLibrary.MakeVector` _x 0.0 _y) (100.0 100.0 100.0)) true))))

(fn `UserConstructionScript`)