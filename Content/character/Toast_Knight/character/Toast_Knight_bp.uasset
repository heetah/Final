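; Toast Knight player character for a fixed-camera, charge-jump platformer, moved by physics forces on its capsule along X and Z.
; Holding Jump builds lift and sideways charge on a looping timer; release launches it if a downward trace finds ground.
; Material parameter collections hold jump charge and HP, with a fail widget at exactly zero HP.
; Escape uses short traces to detect being stuck, then teleports to the last jump-press position.
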(event `self.ReceiveAnyDamage`
  (params (Damage :type "Float (single-precision)") (DamageType :type "DamageType Object Reference") (InstigatedBy :type "Controller Object Reference") (DamageCauser :type "Actor Object Reference"))
  (bind _returnvalue (`KismetMaterialLibrary.GetScalarParameterValue` "/Game/User_Interface/local_DB/TEMP_DATA_local.TEMP_DATA_local" "currenthp"))
  (`KismetMaterialLibrary.SetScalarParameterValue` "/Game/User_Interface/local_DB/TEMP_DATA_local.TEMP_DATA_local" "currenthp" (- _returnvalue Damage))
  (bind _returnvalue_2 (`KismetMaterialLibrary.GetScalarParameterValue` "/Game/User_Interface/local_DB/TEMP_DATA_local.TEMP_DATA_local" "currenthp"))
  (if (== _returnvalue_2 0.0)
    (bind _returnvalue_3 (`|CreateWidget` "/Game/User_Interface/FAIL_.FAIL__C"))
    (`UserWidget.AddToViewport` _returnvalue_3 0)))

(event `self.ReceiveBeginPlay`
  (bind _outactors (`GameplayStatics.GetAllActorsOfClass` "/Game/character/Toast_Knight/character/FixedCamera.FixedCamera_C"))
  (`PlayerController.SetViewTargetWithBlend` (`GameplayStatics.GetPlayerController` 0) (`|GetArrayItem` _outactors) 0.0 "VTBlend_Linear" 0.0 false))

(event `self.ReceiveTick`
  (params (DeltaSeconds :type "Float (single-precision)"))
  (bind _returnvalue (`self.K2_GetActorLocation`))
  (bind (_x _y _z) (`KismetMathLibrary.BreakVector3f` (`self.GetVelocity`)))
  (`PrimitiveComponent.SetAllPhysicsLinearVelocity` (`self.CapsuleComponent`) (`KismetMathLibrary.MakeVector` (`KismetMathLibrary.FClamp` _x -400.0 400.0) _y _z) false)
  (bind (_outhit _returnvalue_2) (`KismetSystemLibrary.LineTraceSingle` _returnvalue (- _returnvalue (0.0 0.0 100.0)) "TraceTypeQuery1"))
  (if _returnvalue_2
    (set `self.IsOnGround` true)
    (else
      (set `self.IsOnGround` false))))

(event `InputAxis|Move_Right`
  (params (AxisValue :type "Float (single-precision)"))
  (if (`self.Is_Jumping`)
    _
    (elif (`self.IsOnGround`)
      (`PrimitiveComponent.AddForce` (`self.CapsuleComponent`) (`KismetMathLibrary.MakeVector` (* AxisValue 1000.0)) "None" true))))

(event `InputAction|Jump`
  (params (Key :type "Key Structure"))
  (:`Pressed`
    (set `self.Prev_Location` (`self.K2_GetActorLocation`))
    (set `self.Is_Jumping` true)
    (bind _returnvalue (`KismetSystemLibrary.K2_SetTimerDelegate` (delegate `ChargeJump`) 0.1 true))
    (set `self.Charge Time Handle` _returnvalue))
  (:`Released`
    (`KismetSystemLibrary.K2_ClearAndInvalidateTimerHandle` (`self.Charge Time Handle`))
    (`KismetSystemLibrary.PrintString` (`KismetStringLibrary.Conv_DoubleToString` (`self.JumpCharge`)) true true (struct :`G` 1.0 :`B` 0.310475 :`A` 1.0))
    (if (`self.IsOnGround`)
      (`PrimitiveComponent.AddForce` (`self.CapsuleComponent`) (`KismetMathLibrary.MakeVector` (`self.RightCharge`) 0.0 (`self.JumpCharge`)) "None" true)
      (`KismetSystemLibrary.PrintString` (`KismetStringLibrary.Conv_DoubleToString` (`self.RightCharge`)) true true (struct :`G` 1.0 :`B` 0.311617 :`A` 1.0))
      (set `self.JumpCharge` 16000.0)
      (set `self.add_charge` 0.0)
      (set `self.Is_Jumping` false)
      (`KismetMaterialLibrary.SetScalarParameterValue` "/Game/User_Interface/Material_for_data/TEMP_DATA.TEMP_DATA" "Charge"))))

(event `ChargeJump`
  (bind _returnvalue (`KismetMathLibrary.FClamp` (+ (`self.JumpCharge`) (`self.add_charge`)) 0.0 60000.0))
  (set `self.RightCharge` (`KismetMathLibrary.FClamp` (+ (`self.RightCharge`) (* (stale `InputAxis|Move_Right` AxisValue) 2000.0)) -20000.0 20000.0))
  (set `self.add_charge` (+ (`self.add_charge`) 1000.0))
  (bind _output_get (set `self.JumpCharge` _returnvalue))
  (`KismetSystemLibrary.PrintString` (`KismetStringLibrary.Conv_DoubleToString` _output_get))
  (`KismetMaterialLibrary.SetScalarParameterValue` "/Game/User_Interface/Material_for_data/TEMP_DATA.TEMP_DATA" "Charge" (/ _returnvalue 60000.0)))

(event `InputAction|Escape`
  (params (Key :type "Key Structure"))
  (:`Pressed`
    (`self.CheckIsStucked`))
  (:`Released`
    (if (`self.IsStucked`)
      (`self.K2_TeleportTo` (`self.Prev_Location`))
      (`PrimitiveComponent.SetAllPhysicsLinearVelocity` (`self.CapsuleComponent`) (0.0 0.0 0.0) false)
      (`KismetSystemLibrary.PrintString` "Escape Suceessfully!!!")
      (else
        (`KismetSystemLibrary.PrintString` "Escape Failed!!!")))))

(fn `CheckIsStucked`
  (bind _returnvalue (`self.K2_GetActorLocation`))
  (bind _returnvalue_2 (`self.K2_GetActorLocation`))
  (bind _returnvalue_3 (`self.K2_GetActorLocation`))
  (bind _returnvalue_4 (`self.K2_GetActorLocation`))
  (set `self.IsStucked` false)
  (bind (_outhit _returnvalue_5) (`KismetSystemLibrary.LineTraceSingle` _returnvalue_2 (+ _returnvalue_2 (10.0 0.0 0.0)) "TraceTypeQuery1"))
  (bind (_outhit_2 _returnvalue_6) (`KismetSystemLibrary.LineTraceSingle` _returnvalue_3 (+ _returnvalue_3 (-10.0 0.0 0.0)) "TraceTypeQuery1"))
  (bind (_outhit_3 _returnvalue_7) (`KismetSystemLibrary.LineTraceSingle` _returnvalue_4 (+ _returnvalue_4 (0.0 0.0 10.0)) "TraceTypeQuery1"))
  (bind (_outhit_4 _returnvalue_8) (`KismetSystemLibrary.LineTraceSingle` _returnvalue (+ _returnvalue (10.0 0.0 -10.0)) "TraceTypeQuery1"))
  (if _returnvalue_5
    (if _returnvalue_6
      (set `self.IsStucked` true)
      (elif _returnvalue_7
        (if _returnvalue_8
          (set `self.IsStucked` true)
          (else
            (`KismetSystemLibrary.PrintString` "Detected No Stucked(1)" true true (struct :`R` 0.998508 :`G` 1.0 :`A` 1.0))))
        (else
          (`KismetSystemLibrary.PrintString` "Detected No Stucked(2)" true true (struct :`R` 0.998508 :`G` 1.0 :`A` 1.0)))))
    (elif _returnvalue_7
      (if true
        (set `self.IsStucked` true)
        (else
          (`KismetSystemLibrary.PrintString` "Detected No Stucked(3)" true true (struct :`R` 0.998508 :`G` 1.0 :`A` 1.0))))
      (else
        (`KismetSystemLibrary.PrintString` "Detected No Stucked(4)" true true (struct :`R` 0.998508 :`G` 1.0 :`A` 1.0))))))

(fn `JumpRelease`)

(fn `UserConstructionScript`)