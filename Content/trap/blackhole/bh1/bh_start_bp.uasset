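; Entrance black hole trap that teleports a character entering its box to a paired Bh_end_bp actor.
; On BeginPlay it picks the exit from all Bh_end_bp actors in the level using the Blackvar index.
; On overlap it moves the character to the exit, keeping its rotation and offset from the entrance.
; A short trailing delay has nothing after it.
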(event `self.ReceiveBeginPlay`
  (bind _outactors (`GameplayStatics.GetAllActorsOfClass` "/Game/trap/blackhole/bh1/bh_end_bp.bh_end_bp_C"))
  (set `self.black2` (`|GetArrayItem` _outactors (`self.blackvar`))))

(event `self.Box.OnComponentBeginOverlap`
  (params (OverlappedComponent :type "PrimitiveComponent Object Reference") (OtherActor :type "Actor Object Reference") (OtherComp :type "PrimitiveComponent Object Reference") (OtherBodyIndex :type Integer) (bFromSweep :type Boolean) (SweepResult :type "HitResult Structure (by ref)"))
  (bind `_as角色` (cast `Character` OtherActor)
    (:`then`
      _)
    (:`CastFailed`
      _))
  (`self.K2_SetActorLocationAndRotation` `_as角色` (- (+ (- (`self.K2_GetActorLocation` `_as角色`) (`self.K2_GetActorLocation`)) (`self.K2_GetActorLocation` (`self.black2`))) (0.0 0.0 0.0)) (`self.K2_GetActorRotation` `_as角色`) false false)
  (`KismetSystemLibrary.Delay` 0.2))

(fn `UserConstructionScript`)